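; Manager Blueprint that controls how many plantable plots in its Plantable array are initialized.
; On BeginPlay it initializes entries up to StartCount or the array length, each pass also disabling Box and Capsule collision at the incremented index.
; AddNewPlot initializes the entry at CurrentCount and increments the counter, with no bounds check or collision change.
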(event EventBeginPlay
  (Variables|Default|SetCurrentCount 0)
  (while (and (< (Variables|Default|GetCurrentCount) (Variables|Default|GetStartCount)) (< (Variables|Default|GetCurrentCount) (Utilities|Array|Length (Variables|Default|GetPlantable))))
    (Default|InitializePlots (Utilities|Array|Get(acopy) (Variables|Default|GetPlantable) (Variables|Default|GetCurrentCount)))
    (Math|Integer|IncrementInt (Variables|Default|GetCurrentCount)
      (:%20%20
        (Collision|SetCollisionEnabled (Variables|/Game/Blueprints/PlantableLand.PlantableLand_C|GetBox (Utilities|Array|Get(acopy) (Variables|Default|GetPlantable) (Variables|Default|GetCurrentCount))) "NoCollision")
        (Collision|SetCollisionEnabled (Variables|/Game/Blueprints/PlantableLand.PlantableLand_C|GetCapsule (Utilities|Array|Get(acopy) (Variables|Default|GetPlantable) (Variables|Default|GetCurrentCount))) "NoCollision")))))

(fn ConstructionScript)

(fn AddNewPlot
  (bind _currentcount (Variables|Default|GetCurrentCount))
  (Default|InitializePlots (Utilities|Array|Get(acopy) (Variables|Default|GetPlantable) _currentcount))
  (Math|Integer|IncrementInt _currentcount))