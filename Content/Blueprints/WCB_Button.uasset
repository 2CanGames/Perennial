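; WCB_Button is a button widget Blueprint that tints its background light red while the first player controller has focus on it, and white otherwise.
; ProcessFocus polls for focus changes against the cached PreviousFocus and calls SetFocusColor only when the state changes.
; A separate NotEveryTick helper uses a tick counter and modulo to return false on every Nth call, though nothing in these graphs calls it.
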(fn NotEveryTick
  (params (TickSkips :type Integer))
  (bind _tickcount (Variables|Default|GettickCount))
  (Math|Integer|IncrementInt _tickcount
    (:%20%20
      (return (not (== (Math|Integer|%(Integer) _tickcount TickSkips) 0))))))

(fn FocusChanged
  (bind _returnvalue (Game|GetPlayerController 0))
  (bind _returnvalue_2 (Class|Widget|HasUserFocus _returnvalue))
  (if (Math|Boolean|Equal(Boolean) (Variables|Default|GetpreviousFocus) _returnvalue_2)
    (return false)
    (else
      (Variables|Default|SetpreviousFocus _returnvalue_2)
      (return true))))

(fn SetFocusColor
  (params (Focus :type Boolean))
  (if Focus
    (Class|Button|SetBackgroundColor "(R=1.000000,G=0.386430,B=0.386430,A=1.000000)")
    (else
      (Class|Button|SetBackgroundColor "(R=1.000000,G=1.000000,B=1.000000,A=1.000000)")))
  (return))

(fn ProcessFocus
  (bind _focuschanged (CallFunction|FocusChanged))
  (if _focuschanged
    (CallFunction|SetFocusColor (Variables|Default|GetpreviousFocus)))
  (return))