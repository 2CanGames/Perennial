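; BP_ComposterActor is a composter actor that shows a floating material billboard while another actor overlaps it.
; Overlap begin and end toggle the billboard's visibility for any actor, with no filtering.
; Tick bobs the billboard vertically by adding a sine of time since creation to its current relative Z, so the motion accumulates per frame and depends on frame rate.
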(event EventBeginPlay)

(event Collision|EventActorBeginOverlap
  (params (OtherActor :type Actor%20Object%20Reference))
  (Rendering|SetVisibility (Variables|Default|GetMaterialBillboard) true true))

(event EventTick
  (params (DeltaSeconds :type Float%20%28single-precision%29))
  (bind _materialbillboard (Variables|Default|GetMaterialBillboard))
  (bind _relativelocation (Variables|/Script/Engine.SceneComponent|GetRelativeLocation _materialbillboard))
  (bind (_x _y _z) (Math|Vector|BreakVector _relativelocation))
  (Transformation|SetRelativeLocation (Variables|Default|GetMaterialBillboard) (Math|Vector|MakeVector _x _y (+ _z (* (Math|Trig|Sin(Radians) (* (Actor|GetGameTimeSinceCreation) 3.0)) 0.2))) false false))

(event Collision|EventActorEndOverlap
  (params (OtherActor :type Actor%20Object%20Reference))
  (Rendering|SetVisibility (Variables|Default|GetMaterialBillboard) false true))

(fn ConstructionScript)