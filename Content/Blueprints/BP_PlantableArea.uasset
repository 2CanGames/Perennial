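; BP_PlantableArea is an actor marking a spot where the player can plant by pressing Q.
; Box overlap events toggle an Interfacable flag, print debug messages and swap the sphere's brown and highlighted materials.
; Begin overlap filters for the player pawn, while end overlap resets for any actor.
; Pressing Q while interactable or overlapping spawns BP_PlantActor at the area's transform and destroys the area.
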(event Custom|OnComponentBeginOverlap_Event_0
  (params (OverlappedComponent :type Primitive%20Component%20Object%20Reference) (OtherActor :type Actor%20Object%20Reference) (OtherComp :type Primitive%20Component%20Object%20Reference) (OtherBodyIndex :type Integer) (bFromSweep :type Boolean) (SweepResult :type Hit%20Result%20Structure%20%28by%20ref%29))
  ;[1 1 1] When the Player Actor enters this item's collision box
  (if (== OtherActor (Game|Player|GetPlayerPawn 0))
    (Variables|Default|SetInterfacable true)
    (Development|PrintString (Utilities|String|Append (Utilities|GetObjectName self) ": Player Enter") true true "(R=0.205750,G=0.014431,B=0.960000,A=1.000000)")
    (Utilities|HighlightMaterial)))

(event Custom|OnComponentEndOverlap_Event_0
  (params (OverlappedComponent :type Primitive%20Component%20Object%20Reference) (OtherActor :type Actor%20Object%20Reference) (OtherComp :type Primitive%20Component%20Object%20Reference) (OtherBodyIndex :type Integer))
  (Variables|Default|SetInterfacable false)
  (Development|PrintString (Utilities|String|Append (Utilities|GetObjectName self) ": Player Exit") true true "(R=0.205750,G=0.014431,B=0.960000,A=1.000000)")
  (Utilities|UnhighlightMaterial))

(event EventBeginPlay
  (bind _box (Variables|Default|GetBox))
  (Collision|AssignOnComponentBeginOverlap _box (delegate Custom|OnComponentBeginOverlap_Event_0))
  (Collision|AssignOnComponentEndOverlap _box (delegate Custom|OnComponentEndOverlap_Event_0))
  (if (Utilities|IsOverlapping)
    (Utilities|HighlightMaterial)
    (else
      (Utilities|UnhighlightMaterial))))

(event Input|KeyboardEvents|Q
  (params (Key :type Key%20Structure :default "AnyKey"))
  (:Pressed
    (if (or (Variables|Default|GetInterfacable) (Utilities|IsOverlapping))
      (Game|SpawnActorfromClass "/Game/Blueprints/BP_PlantActor.BP_PlantActor_C" (Transformation|GetActorTransform) "AlwaysSpawn" 0 0)
      (Actor|DestroyActor))))

(fn ConstructionScript)