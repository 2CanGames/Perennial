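; Seasonal post-process controller that crossfades between spring, summer, fall and winter looks, starting in spring.
; Each Set function marks its season as new and the preceding one as old, assuming a fixed cycle rather than reading the active season.
; While the update flag is set, Tick plays a timeline that drives the two blend weights inversely, then clears the flag and resets its time when finished.
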(event EventBeginPlay
  (Variables|/Script/Engine.PostProcessComponent|SetBlendWeight (Variables|Default|GetPostProcessSpring) 1.0)
  (Variables|/Script/Engine.PostProcessComponent|SetBlendWeight (Variables|Default|GetPostProcessSummer) 0.0)
  (Variables|/Script/Engine.PostProcessComponent|SetBlendWeight (Variables|Default|GetPostProcessWinter) 0.0)
  (Variables|/Script/Engine.PostProcessComponent|SetBlendWeight (Variables|Default|GetPostProcessFall) 0.0))

(event Collision|EventActorBeginOverlap
  (params (OtherActor :type Actor%20Object%20Reference)))

(event EventTick
  (params (DeltaSeconds :type Float%20%28single-precision%29))
  (if (Variables|Default|GetPostProcessUpdated)
    (bind _blendweight (Timeline|Timeline_0 Play)
      (:Update
        (if (Variables|Default|GetPostProcessUpdated)
          (Variables|/Script/Engine.PostProcessComponent|SetBlendWeight (Variables|Default|GetOldPostProcess) _blendweight)
          (Variables|/Script/Engine.PostProcessComponent|SetBlendWeight (Variables|Default|GetNewPostProcess) (- 1.0 _blendweight))))
      (:Finished
        (Variables|Default|SetPostProcessUpdated false)
        (Timeline|Timeline_0 SetNewTime)))))

(fn ConstructionScript)

(fn SetSpring
  (Variables|Default|SetNewPostProcess (Variables|Default|GetPostProcessSpring))
  (Variables|Default|SetOldPostProcess (Variables|Default|GetPostProcessWinter))
  (Variables|Default|SetPostProcessUpdated true)
  (return))

(fn SetSummer
  (Variables|Default|SetNewPostProcess (Variables|Default|GetPostProcessSummer))
  (Variables|Default|SetOldPostProcess (Variables|Default|GetPostProcessSpring))
  (Variables|Default|SetPostProcessUpdated true)
  (return))

(fn SetWinter
  (Variables|Default|SetNewPostProcess (Variables|Default|GetPostProcessWinter))
  (Variables|Default|SetOldPostProcess (Variables|Default|GetPostProcessFall))
  (Variables|Default|SetPostProcessUpdated true)
  (return))

(fn SetFall
  (Variables|Default|SetNewPostProcess (Variables|Default|GetPostProcessFall))
  (Variables|Default|SetOldPostProcess (Variables|Default|GetPostProcessSummer))
  (Variables|Default|SetPostProcessUpdated true)
  (return))