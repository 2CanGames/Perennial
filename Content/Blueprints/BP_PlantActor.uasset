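; Interactable plant-on-plot actor that highlights when the player pawn enters its box and unhighlights when an overlap ends.
; Highlighting swaps slot 0 on the plant and plot meshes between materials stored in each skeletal mesh asset.
; While in range, Q calls DayEnded and refreshes the highlight; the W handler checks range but does nothing.
; Tick bobs the water icon vertically with a sine wave.
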(event Custom|OnComponentBeginOverlap_Event_0
  (params (OverlappedComponent :type Primitive%20Component%20Object%20Reference) (OtherActor :type Actor%20Object%20Reference) (OtherComp :type Primitive%20Component%20Object%20Reference) (OtherBodyIndex :type Integer) (bFromSweep :type Boolean) (SweepResult :type Hit%20Result%20Structure%20%28by%20ref%29))
  ;[1 1 1] When the Player Actor enters this item's collision box
  (if (== OtherActor (Game|Player|GetPlayerPawn 0))
    (Variables|Default|SetInterfacable true)
    (Utilities|HighlightMaterial)))

(event Custom|OnComponentEndOverlap_Event_0
  (params (OverlappedComponent :type Primitive%20Component%20Object%20Reference) (OtherActor :type Actor%20Object%20Reference) (OtherComp :type Primitive%20Component%20Object%20Reference) (OtherBodyIndex :type Integer))
  (Variables|Default|SetInterfacable false)
  (Utilities|UnhighlightMaterial))

(event EventBeginPlay
  (bind _box (Variables|Default|GetBox))
  (Collision|AssignOnComponentBeginOverlap _box (delegate Custom|OnComponentBeginOverlap_Event_0))
  (Collision|AssignOnComponentEndOverlap _box (delegate Custom|OnComponentEndOverlap_Event_0))
  (if (Utilities|IsOverlapping)
    (Utilities|HighlightMaterial)
    (else
      (Utilities|UnhighlightMaterial))))

(event EventTick
  (params (DeltaSeconds :type Float%20%28single-precision%29))
  (bind _watericon (Variables|Default|GetWaterIcon))
  (bind _relativelocation (Variables|/Script/Engine.SceneComponent|GetRelativeLocation _watericon))
  (bind (_x _y _z) (Math|Vector|BreakVector _relativelocation))
  (Transformation|SetRelativeLocation (Variables|Default|GetWaterIcon) (Math|Vector|MakeVector _x _y (+ _z (* (Math|Trig|Sin(Radians) (* (Actor|GetGameTimeSinceCreation) 3.0)) 0.2))) false false))

(event Input|KeyboardEvents|W
  (params (Key :type Key%20Structure :default "AnyKey"))
  (:Pressed
    (if (or (Variables|Default|GetInterfacable) (Utilities|IsOverlapping))
      _)))

(event Input|KeyboardEvents|Q
  (params (Key :type Key%20Structure :default "AnyKey"))
  (:Pressed
    (if (or (Variables|Default|GetInterfacable) (Utilities|IsOverlapping))
      (Class|PlantActor|DayEnded)
      (if (or (Variables|Default|GetInterfacable) (Utilities|IsOverlapping))
        (Utilities|HighlightMaterial)
        (else
          (Utilities|UnhighlightMaterial))))))

(fn ConstructionScript)