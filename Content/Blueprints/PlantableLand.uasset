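; PlantableLand is a land area that fills itself with a line of BP_PlantActor plots.
; InitializePlots hides its Box in game, then calls SetInitPointingLocation to start a cursor just inside the box's minimum-Y edge, centered on X and Z.
; It spawns PlotCount plant actors, advancing the cursor by PlotOffset after each.
; Its event graph is empty, so InitializePlots is not called within this Blueprint.
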(event EventBeginPlay)

(event Collision|EventActorBeginOverlap
  (params (OtherActor :type Actor%20Object%20Reference)))

(event EventTick
  (params (DeltaSeconds :type Float%20%28single-precision%29)))

(fn ConstructionScript)

(fn SetInitPointingLocation
  (bind _box (Variables|Default|GetBox))
  (bind (_origin _boxextent) (Collision|GetComponentBounds _box))
  (Variables|Default|SetPointingLocation (Math|Vector|MakeVector (.x _origin) (+ (- (.y _origin) (.y _boxextent)) 1.5e+02) (+ (.z _origin) 0.0)))
  (return))

(fn InitializePlots
  (Development|SetHiddeninGame (Variables|Default|GetBox) true true)
  (CallFunction|SetInitPointingLocation)
  (bind _output_get (Variables|Default|SetSpawnCount 0))
  (while (< _output_get (Variables|Default|GetPlotCount))
    (bind _returnvalue (Game|SpawnActorfromClass "/Game/Blueprints/BP_PlantActor.BP_PlantActor_C" (Math|Transform|MakeTransform "0, 0,0.000000" "0, 0, 0" "1,1,1") "AlwaysSpawn" 0 0))
    (Transformation|SetActorLocation _returnvalue (Variables|Default|GetPointingLocation) false false)
    (Variables|Default|SetPointingLocation (+ (Variables|Default|GetPointingLocation) (Variables|Default|GetPlotOffset)))
    (Math|Integer|IncrementInt (Variables|Default|GetSpawnCount))))