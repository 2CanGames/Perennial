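; CloudActor is a cloud that drifts endlessly backward along its spline.
; BeginPlay jitters the static mesh's height and picks a random speed and starting distance, so instances vary.
; Each Tick subtracts the speed from the distance, without delta-time scaling, and wraps to the spline's end after reaching the start.
; Only world X and Y follow the spline; the mesh keeps its randomized Z.
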(event EventBeginPlay
  (CallFunction|SetRandomZ)
  (Variables|Default|SetSpeed (Math|Random|RandomFloatinRange 1.0 2.0))
  (bind _output_get (Variables|Default|SetDistanceAlongSpline (Math|Random|RandomFloatinRange 0.0 (Spline|GetSplineLength (Variables|Default|GetSpline)))))
  (CallFunction|SetXYonSpline _output_get))

(event EventTick
  (params (DeltaSeconds :type Float%20%28single-precision%29))
  (if (<= (Variables|Default|GetDistanceAlongSpline) 0.0)
    (Variables|Default|SetDistanceAlongSpline (Spline|GetSplineLength (Variables|Default|GetSpline))))
  (bind _output_get (Variables|Default|SetDistanceAlongSpline (- (Variables|Default|GetDistanceAlongSpline) (Variables|Default|GetSpeed))))
  (CallFunction|SetXYonSpline _output_get))

(fn ConstructionScript)

(fn SetXYonSpline
  (params (Distance :type Float%20%28single-precision%29))
  (bind _spline (Variables|Default|GetSpline))
  (bind _staticmesh (Variables|Default|GetStaticMesh))
  (bind _returnvalue (Spline|GetLocationatDistanceAlongSpline _spline Distance "World"))
  (bind (_x _y) (Math|Vector|BreakVector _returnvalue))
  (Transformation|SetWorldLocation _staticmesh (Math|Vector|MakeVector _x _y (.Z (Math|Vector|BreakVector (Transformation|GetWorldLocation _staticmesh)))) false false))

(fn SetRandomZ
  (bind _staticmesh (Variables|Default|GetStaticMesh))
  (bind _returnvalue (Transformation|GetWorldLocation _staticmesh))
  (bind (_x _y _z) (Math|Vector|BreakVector _returnvalue))
  (Transformation|SetWorldLocation _staticmesh (Math|Vector|MakeVector _x _y (Math|Random|RandomFloatinRange (- _z 1e+02) (+ _z 1e+02))) false false))